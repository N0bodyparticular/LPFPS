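; BP_Cloud is a decorative low-poly cloud that orbits its placement point while spinning.
; Construction offsets the mesh by Radius, randomizes the root yaw and picks a random cloud mesh; one reachable option is empty and the last is never selected.
; Each Tick spins the mesh at SpinRate and yaws the whole actor at MoveSpeed, sweeping the offset cloud around a circle.
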(event `self.ReceiveTick`
  (params (DeltaSeconds :type "Float (single-precision)"))
  (`SceneComponent.K2_AddLocalRotation` (`self.StaticMesh`) (`KismetMathLibrary.MakeRotator` 0.0 0.0 (* DeltaSeconds (`self.SpinRate`))) false false)
  (`self.K2_AddActorWorldRotation` (`KismetMathLibrary.MakeRotator` 0.0 0.0 (* (`GameplayStatics.GetWorldDeltaSeconds`) (`self.MoveSpeed`)))))

(fn `UserConstructionScript`
  (`SceneComponent.K2_AddLocalOffset` (`self.StaticMesh`) (`KismetMathLibrary.MakeVector` (`self.Radius`)) false false)
  (`SceneComponent.K2_SetWorldRotation` (`self.DefaultSceneRoot`) (`KismetMathLibrary.MakeRotator` 0.0 0.0 (`KismetMathLibrary.RandomFloatInRange` 0.0 360.0)) false false)
  (`StaticMeshComponent.SetStaticMesh` (`self.StaticMesh`) (select `int` (`KismetMathLibrary.RandomInteger` 5) :`0` "/Game/Map_Content/Shared/Clouds/LPClouds_Icosphere_004.LPClouds_Icosphere_004" :`1` "/Game/Map_Content/Shared/Clouds/LPClouds_Icosphere_005.LPClouds_Icosphere_005" :`2` "/Game/Map_Content/Shared/Clouds/LPClouds_Icosphere_007.LPClouds_Icosphere_007" :`3` "/Game/Map_Content/Shared/Clouds/LPClouds_Icosphere_010.LPClouds_Icosphere_010" :`4` null :`5` "/Game/Map_Content/Shared/Clouds/LPClouds_Icosphere_013.LPClouds_Icosphere_013" :!type "StaticMesh Object Reference")))