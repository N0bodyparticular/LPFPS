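; First-person testing Character Blueprint with basic walking, jumping and look controls.
; Forward and Right axes feed movement input along the flattened actor vectors, while Tick aligns the camera to the control rotation.
; Look axes sum mouse input with frame-time-scaled controller input, using separate sensitivities and vertical inversion flags.
; The controller term in LookUp reads the LookRightRate axis, same as LookRight.
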(event `InputAxis|Forward`
  (params (AxisValue :type "Float (single-precision)"))
  ;[1 1 1] General movement and input
  (`PawnMovementComponent.AddInputVector` (`self.CharacterMovement`) (* (* (`self.GetActorForwardVector`) (1.0 1.0 0.0)) AxisValue) false))

(event `InputAxis|Right`
  (params (AxisValue :type "Float (single-precision)"))
  ;[1 1 1] General movement and input
  (`PawnMovementComponent.AddInputVector` (`self.CharacterMovement`) (* (* (`self.GetActorRightVector`) (1.0 1.0 0.0)) AxisValue) false))

(event `self.ReceiveTick`
  (params (DeltaSeconds :type "Float (single-precision)"))
  ;[1 1 1] General movement and input
  (`SceneComponent.K2_SetWorldRotation` (`self.Camera`) (`self.GetControlRotation`) false false))

(event `InputAction|Jump`
  (params (Key :type "Key Structure"))
  ;[1 1 1] General movement and input
  (:`Pressed`
    (`self.Jump`))
  (:`Released`
    (`self.StopJumping`)))

(event `InputAxis|LookRight`
  (params (AxisValue :type "Float (single-precision)"))
  ;[1 1 1] General movement and input
  (`self.AddControllerYawInput` (+ (* AxisValue (`self.HorizSens`)) (* (`self.HorizContSens`) (`self.GetInputAxisValue`) (`GameplayStatics.GetWorldDeltaSeconds`)))))

(event `InputAxis|LookUp`
  (params (AxisValue :type "Float (single-precision)"))
  ;[1 1 1] General movement and input
  (`self.AddControllerPitchInput` (+ (* AxisValue (`self.VertSens`) (`KismetMathLibrary.SelectFloat` 1.0 -1.0 (`self.InvertMouseVert`))) (* (`self.VertContSens`) (`self.GetInputAxisValue`) (`GameplayStatics.GetWorldDeltaSeconds`) (`KismetMathLibrary.SelectFloat` 1.0 -1.0 (`self.InvertContVert`))))))

(fn `UserConstructionScript`)